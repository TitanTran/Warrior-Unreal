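; Hero gameplay ability for the axe's heavy special attack, a jump-attack montage with area damage.
; On the AOE gameplay event, a box trace ahead of the hero applies heavy-attack damage scaled from weapon damage at ability level.
; Activation also commits the cooldown and reports it to the hero UI, and the ability ends with the montage.
; A single-target damage function with hit sound and hit-react is defined but not called here.
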(event `self.K2_ActivateAbility`
  (bind _returnvalue (`self.GetHeroCharacterFromActorInfo`))
  (bind _returnvalue_2 (`self.GetCooldownTimeRemaining`))
  (bind _returnvalue_3 (`Actor.K2_GetActorLocation` _returnvalue))
  (bind _returnvalue_4 (`Actor.GetActorForwardVector` _returnvalue))
  (`AbilityTask_PlayMontageAndWait.CreatePlayMontageAndWaitProxy` "None" "/Game/PlayerCharacter/Montages/SpecialWeaponAbility/AM_Hero_Axe_JumpAttack.AM_Hero_Axe_JumpAttack"
    (:`then`
      (`|ExecutionSequence`
        (:`then_0`
          (`AbilityTask_WaitGameplayEvent.WaitGameplayEvent` (struct :`TagName` "Player.Event.AOE") null
            (:`EventReceived`
              (bind _outhits (`KismetSystemLibrary.BoxTraceMultiForObjects` _returnvalue_3 (+ _returnvalue_3 (* _returnvalue_4 200.0)) (300.0 300.0 200.0) (`KismetMathLibrary.Conv_VectorToRotator` _returnvalue_4) (`self.Object Types`)))
              (`self.ApplyGameplayEffectSpecHandleToHitResults` (`self.MakeHeroDamageEffectSpecHandle` "/Game/Shared/GamplayEffect/GE_Shared_DealDamge.GE_Shared_DealDamge_C" (`HeroCombatComponent.GetHeroCurrentEquippWeaponDamageAtLevel` (`self.GetHeroCombatComponentFromActorInfo`) (`KismetMathLibrary.Conv_IntToDouble` (`self.GetAbilityLevel`))) (struct :`TagName` "Player.SetByCaller.AttackType.Heavy") 3) _outhits))))
        (:`then_1`
          (`self.K2_CommitAbilityCooldown` false)
          (`HeroUIComponent.OnAbilityCooldownBegin` (`WarriorHeroCharacter.HeroUIComponent` (`self.GetHeroCharacterFromActorInfo`)) (struct :`TagName` "InputTag.SpecialWeaponAbility.Heavy") _returnvalue_2 _returnvalue_2))))
    (:`OnCompleted`
      (`self.K2_EndAbility` :!label _label))
    (:`OnBlendOut`
      (goto _label))
    (:`OnInterrupted`
      (goto _label))
    (:`OnCancelled`
      (goto _label))))

(fn `HandleApply Damage`
  (params (InPayload :type "GameplayEventData Structure"))
  (locals (CachedTargetActor :type "Actor Object Reference"))
  (bind _output_get (set `local.CachedTargetActor` (`.Target` (break `GameplayEventData` InPayload))))
  (`self.BP_ApplyEffectSpecHandleToTarget` _output_get (`self.MakeHeroDamageEffectSpecHandle` "/Game/Shared/GamplayEffect/GE_Shared_DealDamge.GE_Shared_DealDamge_C" (`HeroCombatComponent.GetHeroCurrentEquippWeaponDamageAtLevel` (`self.GetHeroCombatComponentFromActorInfo`) (`KismetMathLibrary.Conv_IntToDouble` (`self.GetAbilityLevel`))) (struct :`TagName` "Player.SetByCaller.AttackType.Light") 4)
    (:`Successful`
      (`self.K2_ExecuteGameplayCue` (struct :`TagName` "GameplayCue.Sounds.MeleeHit.Axe"))
      (`AbilitySystemBlueprintLibrary.SendGameplayEventToActor` (`local.CachedTargetActor`) (struct :`TagName` "Shared.Event.HitReact") (`local.InPayload`)))))