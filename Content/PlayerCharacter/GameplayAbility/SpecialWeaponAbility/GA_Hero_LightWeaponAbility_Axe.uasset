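; Hero gameplay ability for the axe's light special weapon attack.
; It plays the attack montage while waiting for a melee hit event, commits the cooldown and notifies the hero UI.
; A hit applies weapon-based damage as a light attack with a fixed combo count, then on success fires the axe hit sound cue and sends a hit react event to the target.
; The ability ends when the montage finishes or is interrupted.
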(event `self.K2_ActivateAbility`
  (bind _returnvalue (`self.GetCooldownTimeRemaining`))
  (`AbilityTask_PlayMontageAndWait.CreatePlayMontageAndWaitProxy` "None" "/Game/PlayerCharacter/Montages/SpecialWeaponAbility/AM_Hero_Axe_Ability_Light.AM_Hero_Axe_Ability_Light"
    (:`then`
      (`|ExecutionSequence`
        (:`then_0`
          (bind (_asynctaskproxy _payload) (`AbilityTask_WaitGameplayEvent.WaitGameplayEvent` (struct :`TagName` "Shared.Event.MeleeHit") null)
            (:`EventReceived`
              (`self.HandleApply Damage` _payload))))
        (:`then_1`
          (`self.K2_CommitAbilityCooldown` false)
          (`HeroUIComponent.OnAbilityCooldownBegin` (`WarriorHeroCharacter.HeroUIComponent` (`self.GetHeroCharacterFromActorInfo`)) (struct :`TagName` "InputTag.SpecialWeaponAbility.Light") _returnvalue _returnvalue))))
    (:`OnCompleted`
      (`self.K2_EndAbility` :!label _label))
    (:`OnBlendOut`
      (goto _label))
    (:`OnInterrupted`
      (goto _label))
    (:`OnCancelled`
      (goto _label))))

(fn `HandleApply Damage`
  (params (InPayload :type "GameplayEventData Structure"))
  (locals (CachedTargetActor :type "Actor Object Reference"))
  (bind _output_get (set `local.CachedTargetActor` (`.Target` (break `GameplayEventData` InPayload))))
  (`self.BP_ApplyEffectSpecHandleToTarget` _output_get (`self.MakeHeroDamageEffectSpecHandle` "/Game/Shared/GamplayEffect/GE_Shared_DealDamge.GE_Shared_DealDamge_C" (`HeroCombatComponent.GetHeroCurrentEquippWeaponDamageAtLevel` (`self.GetHeroCombatComponentFromActorInfo`) (`KismetMathLibrary.Conv_IntToDouble` (`self.GetAbilityLevel`))) (struct :`TagName` "Player.SetByCaller.AttackType.Light") 4)
    (:`Successful`
      (`self.K2_ExecuteGameplayCue` (struct :`TagName` "GameplayCue.Sounds.MeleeHit.Axe"))
      (`AbilitySystemBlueprintLibrary.SendGameplayEventToActor` (`local.CachedTargetActor`) (struct :`TagName` "Shared.Event.HitReact") (`local.InPayload`)))))